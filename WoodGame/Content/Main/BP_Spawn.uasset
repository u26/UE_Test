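; Spawner actor that emits a burst of BP_Ball actors from its Arrow's location and rotation when EventSpawnBall is called.
; The event spawns one ball immediately and starts a looping timer that re-enters the same spawn logic at each SpawnInterval.
; Each ball receives the supplied velocity, a reduced supplied scale and a SpawnMaskDelay wait.
; A counter stops the timer and resets once GenerateNum balls have spawned.
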(event Custom|EventSpawnBall
  (params (BP_Ball :type BP%20Ball%20Object%20Reference) (velocity :type Vector) (scale :type Vector))
  (bind _arrow (Variables|Default|GetArrow))
  (bind _returnvalue (Transformation|GetWorldTransform _arrow))
  (bind _returnvalue_2 (Utilities|Time|SetTimerbyEvent (delegate Custom|CustomEvent_0) (Variables|Default|Getspawn_interval) true))
  (Variables|Default|Settimer _returnvalue_2)
  (Math|Integer|IncrementInt (Variables|Default|Getcnt)
    (:%20%20
      (if (<= (Variables|Default|Getcnt) (Variables|Default|Getgenerate_num))
        (Game|SpawnActorfromClass "/Game/Main/BP_Ball.BP_Ball_C" (Math|Transform|MakeTransform (.location _returnvalue) (.rotation _returnvalue) (* scale 0.75)) "Undefined" 0 true velocity (Variables|Default|Getspawn_mask_delay) 0)
        (else
          (Variables|Default|Setcnt 0)
          (Utilities|Time|ClearandInvalidateTimerbyHandle (Variables|Default|Gettimer)))))))

(event Custom|CustomEvent_0
  (bind _arrow (Variables|Default|GetArrow))
  (bind _returnvalue (Transformation|GetWorldTransform _arrow))
  (Math|Integer|IncrementInt (Variables|Default|Getcnt)
    (:%20%20
      (if (<= (Variables|Default|Getcnt) (Variables|Default|Getgenerate_num))
        (Game|SpawnActorfromClass "/Game/Main/BP_Ball.BP_Ball_C" (Math|Transform|MakeTransform (.location _returnvalue) (.rotation _returnvalue) (* (stale Custom|EventSpawnBall scale) 0.75)) "Undefined" 0 true (stale Custom|EventSpawnBall velocity) (Variables|Default|Getspawn_mask_delay) 0)
        (else
          (Variables|Default|Setcnt 0)
          (Utilities|Time|ClearandInvalidateTimerbyHandle (Variables|Default|Gettimer)))))))

(event EventBeginPlay)

(event Collision|EventActorBeginOverlap
  (params (OtherActor :type Actor%20Object%20Reference)))

(event EventTick
  (params (DeltaSeconds :type Float%20%28single-precision%29)))

(fn ConstructionScript)