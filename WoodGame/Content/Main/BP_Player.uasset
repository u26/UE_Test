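; Player pawn with look and movement input that can grab, carry, throw and poke physics objects.
; A camera line trace finds PhysicsBody objects for grabbing or poking.
; Grab snaps HeldObjectSlot to the object, joins them with a physics constraint, then eases the slot to its default hold position, adjustable by mouse wheel.
; Poke applies a camera-forward impulse, first releasing any held object to launch it.
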(event EventBeginPlay)

(event Collision|EventActorBeginOverlap
  (params (OtherActor :type Actor%20Object%20Reference)))

(event EventTick
  (params (DeltaSeconds :type Float%20%28single-precision%29)))

(event Input|ActionEvents|InputActionGrab
  (params (Key :type Key%20Structure))
  (bind _heldobjectslot (Variables|Default|GetHeldObjectSlot))
  ;[1 1 1] Grab
  (:Pressed
    (Utilities|IsValid (Variables|Default|GetHeldObject)
      (:Is%20Valid
        (CallFunction|DropObject)
        (Variables|Default|SetHeldObject 0))
      (:Is%20Not%20Valid
        (bind (_hit_reulst _hit) (CallFunction|TraceObject))
        (if _hit
          (CallFunction|GrabObject _hit_reulst)
          (Components|MoveComponentTo _heldobjectslot (Variables|/Script/Engine.SceneComponent|GetRelativeLocation (Variables|Default|GetHeldObjectDefaultLocation)) (Variables|/Script/Engine.SceneComponent|GetRelativeRotation _heldobjectslot) true true 0.3 false))))))

(event Input|ActionEvents|InputActionPoke
  (params (Key :type Key%20Structure))
  (:Pressed
    (Utilities|IsValid (Variables|Default|GetHeldObject)
      (:Is%20Valid
        ;[1 1 1] Grabbed and Poke
        (CallFunction|DropObject)
        (CallFunction|PokeObject (Collision|MakeHitResult false false 0.0 0.0 "0, 0, 0" (Transformation|GetWorldLocation (Variables|Default|GetHeldObject)) "0,0,1" "0,0,1" 0 0 (Variables|Default|GetHeldObject)))
        (Variables|Default|SetHeldObject 0))
      (:Is%20Not%20Valid
        ;[1 1 1] Poke
        (bind _hit_reulst (CallFunction|TraceObject))
        (CallFunction|PokeObject _hit_reulst)))))

(event Input|AxisEvents|InputAxisLookUp
  (params (AxisValue :type Float%20%28single-precision%29))
  ;[1 1 1] 視線：上下左右
  (Pawn|Input|AddControllerPitchInput AxisValue))

(event Input|AxisEvents|InputAxisTurn
  (params (AxisValue :type Float%20%28single-precision%29))
  ;[1 1 1] 視線：上下左右
  (Pawn|Input|AddControllerYawInput AxisValue))

(event Input|AxisEvents|InputAxisLR
  (params (AxisValue :type Float%20%28single-precision%29))
  ;[1 1 1] 移動：上下左右
  (Pawn|Input|AddMovementInput (Transformation|GetActorRightVector) AxisValue false))

(event Input|AxisEvents|InputAxisFwRw
  (params (AxisValue :type Float%20%28single-precision%29))
  ;[1 1 1] 移動：上下左右
  (Pawn|Input|AddMovementInput (Transformation|GetActorForwardVector) AxisValue false))

(event Input|MouseEvents|MouseWheelUp
  (params (Key :type Key%20Structure))
  ;[1 1 1] Move grabbed Object Near/Far
  (:Pressed
    (Transformation|SetRelativeLocation (Variables|Default|GetHeldObjectSlot) (+ (Variables|/Script/Engine.SceneComponent|GetRelativeLocation (Variables|Default|GetHeldObjectSlot)) "50.000000, 0, 0") false false)))

(event Input|MouseEvents|MouseWheelDown
  (params (Key :type Key%20Structure))
  (bind _heldobjectslot (Variables|Default|GetHeldObjectSlot))
  ;[1 1 1] Move grabbed Object Near/Far
  (:Pressed
    (Transformation|SetRelativeLocation _heldobjectslot (+ (Variables|/Script/Engine.SceneComponent|GetRelativeLocation _heldobjectslot) "-50.000000, 0, 0") false false)))

(fn ConstructionScript)

(fn TraceObject
  (bind _camera (Variables|Default|GetCamera))
  (bind _returnvalue (Transformation|GetWorldLocation _camera))
  (bind (_outhit _returnvalue_2) (Collision|LineTraceForObjects _returnvalue (+ _returnvalue (* (Math|Vector|GetForwardVector _camera) (Variables|Default|GetinterructionDistance))) (Utilities|Array|MakeArray "ObjectTypeQuery4") false 0 "None"))
  (return _outhit _returnvalue_2))

(fn DropObject
  (Class|PhysicsConstraintComponent|BreakConstraint (Variables|Default|GetGrabConstraint))
  (Collision|SetCollisionResponsetoChannel (Variables|Default|GetHeldObjectSlot) "ECC_Pawn" "ECR_Block"))

(fn GrabObject
  (params (HitResult :type Hit%20Result%20Structure))
  (bind (_bblockinghit _binitialoverlap _time _distance _location _impactpoint _normal _impactnormal _physmat _hitactor _hitcomponent _hitbonename) (Collision|BreakHitResult HitResult))
  (Transformation|SetWorldLocation (Variables|Default|GetHeldObjectSlot) (Transformation|GetActorLocation _hitactor) false false)
  (Class|PhysicsConstraintComponent|SetConstrainedComponents (Variables|Default|GetGrabConstraint) (Variables|Default|GetHeldObjectSlot) "None" _hitcomponent _hitbonename)
  (Collision|SetCollisionResponsetoChannel _hitcomponent "ECC_Pawn" "ECR_Block")
  (Variables|Default|SetHeldObject _hitcomponent))

(fn PokeObject
  (params (HitResult :type Hit%20Result%20Structure))
  (bind (_bblockinghit _binitialoverlap _time _distance _location _impactpoint _normal _impactnormal _physmat _hitactor _hitcomponent _hitbonename) (Collision|BreakHitResult HitResult))
  (Physics|AddImpulseatLocation _hitcomponent (* (Math|Vector|GetForwardVector (Variables|Default|GetCamera)) (Variables|Default|GetPower)) _impactpoint _hitbonename))