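; BP_Spawn is a spawner actor that launches a numbered series of BP_Ball actors from its own transform.
; EventSpawnBall, guarded against re-entry by Generating, spawns one ball immediately, then repeats on a looping timer until GenerateNum is reached and clears it.
; SpawnBall passes each ball its number and gives its Sphere a velocity-change impulse along the spawner's forward vector with a random offset.
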(event Custom|EventSpawnBall
  (if (not (Variables|Default|Getgenerating))
    (Variables|Default|Setgenerating true)
    (bind _returnvalue (Utilities|Time|SetTimerbyEvent (delegate Custom|TimerCallback) (Variables|Default|Getgenerate_interval) true))
    (Variables|Default|Settimer _returnvalue)
    (Variables|Default|Setcnt 0)
    (Math|Integer|IncrementInt (Variables|Default|Getcnt)
      (:%20%20
        (if (<= (Variables|Default|Getcnt) (Variables|Default|Getgenerate_num))
          (CallFunction|SpawnBall (Variables|Default|Getcnt))
          (else
            (Utilities|Time|ClearandInvalidateTimerbyHandle (Variables|Default|Gettimer))
            (Variables|Default|Setgenerating false)))))))

(event Custom|TimerCallback
  (Math|Integer|IncrementInt (Variables|Default|Getcnt)
    (:%20%20
      (if (<= (Variables|Default|Getcnt) (Variables|Default|Getgenerate_num))
        (CallFunction|SpawnBall (Variables|Default|Getcnt))
        (else
          (Utilities|Time|ClearandInvalidateTimerbyHandle (Variables|Default|Gettimer))
          (Variables|Default|Setgenerating false))))))

(event EventBeginPlay)

(event Collision|EventActorBeginOverlap
  (params (OtherActor :type Actor%20Object%20Reference)))

(event EventTick
  (params (DeltaSeconds :type Float%20%28single-precision%29)))

(fn ConstructionScript)

(fn SpawnBall
  (params (no :type Integer))
  (bind _returnvalue (Transformation|GetActorTransform))
  (bind _returnvalue_2 (Game|SpawnActorfromClass "/Game/Main/BP_Ball.BP_Ball_C" (Math|Transform|MakeTransform (.location _returnvalue) (.rotation _returnvalue) (* (Variables|Default|GetSpawn%20Transform%20Scale) "1.000000,1.000000,1.000000")) "Undefined" 0 no 0))
  (Physics|AddImpulse (Variables|/Game/Main/BP_Ball.BP_Ball_C|GetSphere _returnvalue_2) (+ (* (Transformation|GetActorForwardVector) (Variables|Default|GetVelocity)) (Math|Random|RandomFloatinRange -5e+01 5e+01)) "None" true))