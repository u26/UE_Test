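; First-person player character with axis-driven look and movement, plus the ability to pick up physics objects.
; Pressing Fire line-traces from the camera against PhysicsBody objects, or drops whatever is already held.
; Grabbing moves HeldObjectSlot to the impact point and joins it to the hit component through GrabConstraint, a physics constraint that dropping breaks.
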(event EventBeginPlay)

(event Collision|EventActorBeginOverlap
  (params (OtherActor :type Actor%20Object%20Reference)))

(event EventTick
  (params (DeltaSeconds :type Float%20%28single-precision%29)))

(event Input|ActionEvents|InputActionFire
  (params (Key :type Key%20Structure :default "None"))
  (:Pressed
    (Utilities|IsValid (Variables|Default|GetHeldObject)
      (:Is%20Valid
        (CallFunction|DropObject))
      (:Is%20Not%20Valid
        (bind (_hit_reulst _hit) (CallFunction|TraceObject))
        (if _hit
          (CallFunction|GrabObject _hit_reulst))))))

(event Input|AxisEvents|InputAxisLookUp
  (params (AxisValue :type Float%20%28single-precision%29))
  ;[1 1 1] 視線：上下左右
  (Pawn|Input|AddControllerPitchInput AxisValue))

(event Input|AxisEvents|InputAxisTurn
  (params (AxisValue :type Float%20%28single-precision%29))
  ;[1 1 1] 視線：上下左右
  (Pawn|Input|AddControllerYawInput AxisValue))

(event Input|AxisEvents|InputAxisLR
  (params (AxisValue :type Float%20%28single-precision%29))
  ;[1 1 1] 移動：上下左右
  (Pawn|Input|AddMovementInput (Transformation|GetActorRightVector) AxisValue false))

(event Input|AxisEvents|InputAxisFwRw
  (params (AxisValue :type Float%20%28single-precision%29))
  ;[1 1 1] 移動：上下左右
  (Pawn|Input|AddMovementInput (Transformation|GetActorForwardVector) AxisValue false))

(fn ConstructionScript)

(fn TraceObject
  (bind _camera (Variables|Default|GetCamera))
  (bind _returnvalue (Transformation|GetWorldLocation _camera))
  (bind (_outhit _returnvalue_2) (Collision|LineTraceForObjects _returnvalue (+ _returnvalue (* (Math|Vector|GetForwardVector _camera) (Variables|Default|GetinterructionDistance))) (Utilities|Array|MakeArray "ObjectTypeQuery4") false 0 "None"))
  (return _outhit _returnvalue_2))

(fn DropObject
  (Class|PhysicsConstraintComponent|BreakConstraint (Variables|Default|GetGrabConstraint))
  (Collision|SetCollisionResponsetoChannel (Variables|Default|GetHeldObjectSlot) "ECC_Pawn" "ECR_Block")
  (Variables|Default|SetHeldObject 0))

(fn GrabObject
  (params (HitResult :type Hit%20Result%20Structure))
  (bind (_bblockinghit _binitialoverlap _time _distance _location _impactpoint _normal _impactnormal _physmat _hitactor _hitcomponent _hitbonename) (Collision|BreakHitResult HitResult))
  (Transformation|SetWorldLocation (Variables|Default|GetHeldObjectSlot) _impactpoint false false)
  (Class|PhysicsConstraintComponent|SetConstrainedComponents (Variables|Default|GetGrabConstraint) (Variables|Default|GetHeldObjectSlot) "None" _hitcomponent _hitbonename)
  (Collision|SetCollisionResponsetoChannel _hitcomponent "ECC_Pawn" "ECR_Block")
  (Variables|Default|SetHeldObject _hitcomponent))